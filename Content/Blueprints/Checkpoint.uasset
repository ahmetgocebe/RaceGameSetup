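; Checkpoint actor that registers a vehicle passing through it in the correct direction.
; When a VehicleBlueprint leaves the trigger, a dot product of its velocity and the arrow's forward vector confirms the travel direction.
; A valid pass broadcasts the checkpoint number as cleared, hides the particle effect and disables further overlap events, so each checkpoint clears only once.
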(event `self.Trigger.OnComponentEndOverlap`
  (params (OverlappedComponent :type "PrimitiveComponent Object Reference") (OtherActor :type "Actor Object Reference") (OtherComp :type "PrimitiveComponent Object Reference") (OtherBodyIndex :type Integer))
  ;[1 1 1] Check Point System-Cleared When Overlapping Ends
  (bind _asvehicle_blueprint (cast `/Game/VehicleAdvBP/Blueprints/VehicleBlueprint` OtherActor))
  (if (> (`KismetMathLibrary.Dot_VectorVector` (`self.GetVelocity` _asvehicle_blueprint) (`KismetMathLibrary.Conv_RotatorToVector` (`SceneComponent.K2_GetComponentRotation` (`self.Arrow`)))) 0.0)
    (`self.CheckpointCleared` (`self.CheckPointNumber`))
    (`SceneComponent.SetHiddenInGame` (`self.ParticleSystem`) true false)
    (set `PrimitiveComponent.bGenerateOverlapEvents` false (`self.Trigger`)) ; collision will not work after this
  ))

(fn `UserConstructionScript`)